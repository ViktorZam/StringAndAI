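; AI dragon character that spawns with a sound and aura effect, then moves toward a target actor through one of three movement events.
; V1 moves directly, V2 drives walk speed from a timeline, and V3 alternates between target and Home using timelines as timers until it arrives.
; On successful arrival, each event calls Finish on the BP_TargetForAI target, with V2 and V3 also stopping their timelines.
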(event Custom|StartAIMovingV3
  (params (TargetActor :type Actor%20Object%20Reference) (Home :type Actor%20Object%20Reference))
  ;[1 1 1] Moving AI
  (AI|AIMoveTo self "0, 0, 0" TargetActor 1e+02 false :!label _label
    (:then
      (Timeline|MovingForward_Timeline PlayFromStart
        (:Finished
          (AI|AIMoveTo self "0, 0, 0" Home 1e+02 false
            (:then
              (Timeline|BackMoving_Timeline PlayFromStart
                (:Finished
                  (goto _label))))))))
    (:OnSuccess
      (CallFunction|StopTimeLines)
      (bind _asbp_target_for_ai (Utilities|Casting|CastToBP_TargetForAI TargetActor))
      (Default|Finish _asbp_target_for_ai))))

(event Custom|StartAIMovingV1
  (params (TargetActor :type Actor%20Object%20Reference))
  ;[1 1 1] Moving AI
  (AI|AIMoveTo self "0, 0, 0" TargetActor 1e+02 false
    (:OnSuccess
      (bind _asbp_target_for_ai (Utilities|Casting|CastToBP_TargetForAI TargetActor))
      (Default|Finish _asbp_target_for_ai))))

(event Custom|StartAIMovingV2
  (params (TargetActor :type Actor%20Object%20Reference))
  ;[1 1 1] Moving AI
  (AI|AIMoveTo self "0, 0, 0" TargetActor 1e+02 false
    (:then
      (bind _speedai (Timeline|Stop/Run_Timeline PlayFromStart)
        (:Update
          (Variables|/Script/Engine.CharacterMovementComponent|SetMaxWalkSpeed (Variables|Character|GetCharacterMovement) _speedai))))
    (:OnSuccess
      (Audio|Components|Audio|Stop (Variables|Default|GetStop/Run_Timeline))
      (bind _asbp_target_for_ai (Utilities|Casting|CastToBP_TargetForAI TargetActor))
      (Default|Finish _asbp_target_for_ai))))

(event Custom|StopTimeLines
  ;[1 1 1] Moving AI
  ;;[1 1 1] Stop Timelines
  (Audio|Components|Audio|Stop (Variables|Default|GetMovingForward_Timeline))
  (Audio|Components|Audio|Stop (Variables|Default|GetBackMoving_Timeline)))

(event EventBeginPlay
  (Audio|SpawnSound2D "/Game/MyContent/Sounds/Cue/DragonBorn_Cue.DragonBorn_Cue" 0.6 1.5 0.0 0)
  (Effects|SpawnEmitteratLocation "/Game/MyContent/Assets/FX/P_Aura_Default_Ending.P_Aura_Default_Ending" (Transformation|GetActorLocation) (Transformation|GetActorRotation)))

(fn ConstructionScript)
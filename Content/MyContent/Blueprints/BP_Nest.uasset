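; BP_Nest is a spawn point that creates AI dragon characters and starts their movement.
; Its SpawnAI event spawns a BP_AI_DragonCharacter at the nest's location and rotation.
; The nest's first actor tag selects one of three movement versions, each given TargetForAI as its target.
; The third version also receives the nest itself as the dragon's home.
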(event Custom|SpawnAI
  ;[1 1 1] Spawn and control AI
  (bind _returnvalue (AI|SpawnAIFromClass "/Game/MyContent/Blueprints/AI/BP_AI_DragonCharacter.BP_AI_DragonCharacter_C" 0 (Transformation|GetActorLocation) (Transformation|GetActorRotation) false 0))
  (bind _asbp_ai_dragon_character (Utilities|Casting|CastToBP_AI_DragonCharacter _returnvalue))
  (switch name (Utilities|Array|Get(acopy) (Variables|Actor|GetTags))
    (:1
      (Default|StartAIMovingV1 _asbp_ai_dragon_character (Variables|Default|GetTargetForAI)))
    (:2
      (Default|StartAIMovingV2 _asbp_ai_dragon_character (Variables|Default|GetTargetForAI)))
    (:3
      (Default|StartAIMovingV3 _asbp_ai_dragon_character (Variables|Default|GetTargetForAI) self))))

(event EventBeginPlay)

(fn ConstructionScript)